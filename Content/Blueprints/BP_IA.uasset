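; BP_IA adds push-to-talk AI conversation to its owning BP_ThirdPersonCharacter, turning recorded player voice into NPC subtitles.
; Holding IA_RecordAudio runs the character's AudioCapture into the Record submix, and releasing exports a WAV file.
; After a short fixed delay, it POSTs a JSON HTTP request using its Url and Body variables.
; The response's transcription and NPC reply fields feed the HUD's subtitle widget.
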(event `self.ReceiveBeginPlay`
  ; Get Player Class
  (bind _asbp_third_person_character (cast `/Game/ThirdPerson/Blueprints/BP_ThirdPersonCharacter` (`self.GetOwner`)))
  (set `self.Player BP` _asbp_third_person_character))

(event `EnhancedInput|/Game/ThirdPerson/Input/Actions/IA_RecordAudio`
  (params (ActionValue :type Boolean) (ElapsedSeconds :type "Float (double-precision)") (TriggeredSeconds :type "Float (double-precision)") (InputAction :type "InputAction Object Reference" :default "/Game/ThirdPerson/Input/Actions/IA_RecordAudio.IA_RecordAudio"))
  (bind _audiocapture (`/Game/ThirdPerson/Blueprints/BP_ThirdPersonCharacter.AudioCapture` (`self.Player BP`)))
  ;[0.05729 0.05729 0.05729 0.5] Audio Record
  (:`Started`
    (`SynthComponent.Start` _audiocapture)
    (`AudioMixerBlueprintLibrary.StartRecordingOutput` 0.0 "/Game/Sounds/Record.Record")
    (`KismetSystemLibrary.PrintString` "Recording..." true true (struct :`R` 1.0 :`A` 1.0) 3.0))
  (:`Completed`
    (`SynthComponent.Stop` _audiocapture)
    (`AudioMixerBlueprintLibrary.StopRecordingOutput` "WavFile" "Record" "" "/Game/Sounds/Record.Record" null)
    (`KismetSystemLibrary.PrintString` "Finish recording" true true (struct :`R` 1.0 :`A` 1.0) 2.0 "1")
    (`KismetSystemLibrary.Delay` 0.1)
    (bind (_outheader _result_body) (`|HttpRequest` (`self.Url`) "Post" (`|MakeRequestHeader` "Json") (`self.Body`))
      (:`On Success`
        (bind _outjsonobject (`JsonBlueprintFunctionLibrary.FromString` _result_body))
        (`|ExecutionSequence`
          (:`then_0`
            (bind _outvalue (`|GetJsonField` _outjsonobject "transcription"))
            (bind _asbp_hud (cast `/Game/UI/BP_HUD` (`PlayerController.GetHUD` (`GameplayStatics.GetPlayerController` 0))))
            (`/Game/UI/WB_Subtitle.SetTranscription` (`/Game/UI/WB_HUD.WB_Subtitle` (`/Game/UI/BP_HUD.UI_Ref` _asbp_hud)) _outvalue 0.0))
          (:`then_1`
            (bind _outvalue_2 (`|GetJsonField` _outjsonobject "npc_response"))
            (bind _asbp_hud_2 (cast `/Game/UI/BP_HUD` (`PlayerController.GetHUD` (`GameplayStatics.GetPlayerController` 0))))
            (`/Game/UI/WB_Subtitle.SetSubtitle` (`/Game/UI/WB_HUD.WB_Subtitle` (`/Game/UI/BP_HUD.UI_Ref` _asbp_hud_2)) _outvalue_2 10.0)))))))